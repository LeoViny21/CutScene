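; BP_NPC is an NPC that plays a hand-off cinematic when the player enters its Box trigger.
; It caches the player's BP_ThirdPersonCharacter on BeginPlay and reacts only to overlaps from that actor.
; Each such overlap creates and plays an SQ_HandOff sequence player, then passes player, NPC and SM_ChamferCube mesh to BPCUpdateObject's UpdateObject.
; Nothing guards against retriggering on re-entry.
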(event OnComponentBeginOverlap(Box)
  (params (OverlappedComponent :type Primitive%20Component%20Object%20Reference) (OtherActor :type Actor%20Object%20Reference) (OtherComp :type Primitive%20Component%20Object%20Reference) (OtherBodyIndex :type Integer) (bFromSweep :type Boolean) (SweepResult :type Hit%20Result%20Structure%20%28by%20ref%29))
  (if (== (Variables|Default|GetAs%20BP%20Third%20Person%20Character) OtherActor)
    (bind _outactor (Sequencer|Player|CreateLevelSequencePlayer "/Game/Blueprint/Character/SQ_HandOff.SQ_HandOff" (Utilities|Struct|MakeMovieSceneSequencePlaybackSettings true "(Value=0)")))
    (Sequencer|Player|Play (Variables|/Script/LevelSequence.LevelSequenceActor|GetSequencePlayer _outactor) :!class /Script/MovieScene.MovieSceneSequencePlayer)
    (Default|UpdateObject (Variables|Default|GetBPC_UpdateObject) (Variables|Default|GetAs%20BP%20Third%20Person%20Character) self "/Game/LevelPrototyping/Meshes/SM_ChamferCube.SM_ChamferCube")))

(event EventBeginPlay
  (bind _asbp_third_person_character (Utilities|Casting|CastToBP_ThirdPersonCharacter (Game|GetPlayerCharacter 0)))
  (Variables|Default|SetAs%20BP%20Third%20Person%20Character _asbp_third_person_character))

(event Collision|EventActorBeginOverlap
  (params (OtherActor :type Actor%20Object%20Reference)))

(event EventTick
  (params (DeltaSeconds :type Float%20%28single-precision%29)))

(fn ConstructionScript)