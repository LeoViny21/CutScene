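; BP_WeaponPickup is a world pickup actor that hands its weapon to the player when walked over.
; BeginPlay caches the player's BP_ThirdPersonCharacter.
; When that character overlaps the Box, it passes the StaticMesh component's mesh to BPCItemPickup's PickUpWeapon, then destroys itself.
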(event OnComponentBeginOverlap(Box)
  (params (OverlappedComponent :type Primitive%20Component%20Object%20Reference) (OtherActor :type Actor%20Object%20Reference) (OtherComp :type Primitive%20Component%20Object%20Reference) (OtherBodyIndex :type Integer) (bFromSweep :type Boolean) (SweepResult :type Hit%20Result%20Structure%20%28by%20ref%29))
  (bind _as_bp_third_person_character (Variables|Default|GetAs%20BP%20Third%20Person%20Character))
  (if (== _as_bp_third_person_character OtherActor)
    (Default|PickUpWeapon (Variables|Default|GetBPC_ItemPickup) _as_bp_third_person_character (Variables|/Script/Engine.StaticMeshComponent|GetStaticMesh (Variables|Default|GetStaticMesh)))
    (Actor|DestroyActor)))

(event EventBeginPlay
  (bind _asbp_third_person_character (Utilities|Casting|CastToBP_ThirdPersonCharacter (Game|GetPlayerCharacter 0)))
  (Variables|Default|SetAs%20BP%20Third%20Person%20Character _asbp_third_person_character))

(event Collision|EventActorBeginOverlap
  (params (OtherActor :type Actor%20Object%20Reference)))

(event EventTick
  (params (DeltaSeconds :type Float%20%28single-precision%29)))

(fn ConstructionScript)