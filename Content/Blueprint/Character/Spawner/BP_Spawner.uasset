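; BP_Spawner is a spawner actor that spawns a set of actors when play begins.
; BeginPlay calls SpawnActors, which loops over TempItemArray and passes each class to the SpawnActor function.
; That function places each actor 100 units above the world origin location returned by GetWorldOriginLocation, with a random integer offset of up to 100 units on X and Y.
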(event Custom|Spawn%20Actors
  (for _array_element (Variables|Default|GetTempItemArray)
    (CallFunction|SpawnActor _array_element)))

(event EventBeginPlay
  (CallFunction|SpawnActors))

(event Collision|EventActorBeginOverlap
  (params (OtherActor :type Actor%20Object%20Reference)))

(event EventTick
  (params (DeltaSeconds :type Float%20%28single-precision%29)))

(fn ConstructionScript)

(fn SpawnActor
  (params (ActorInput :type Actor%20Class%20Reference))
  (bind _returnvalue (Class|GameplayStatics|GetWorldOriginLocation))
  (bind _returnvalue_2 (Math|Random|RandomIntegerinRange -100 100))
  (Game|SpawnActorfromClass ActorInput (Math|Transform|MakeTransform (Math|Vector|MakeVector (Math|Conversions|ToFloat(Integer) (+ (.x _returnvalue) _returnvalue_2)) (Math|Conversions|ToFloat(Integer) (+ (.y _returnvalue) _returnvalue_2)) (Math|Conversions|ToFloat(Integer) (+ (.z _returnvalue) 100))) "0, 0, 0" "1.000000,1.000000,1.000000") "Undefined" "MultiplyWithRoot" 0 0)
  (return))